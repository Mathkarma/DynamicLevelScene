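; BP_DynamicCube is a grid spawner that lays out a square field of BP_Cube child actors in its construction script.
; Nested loops add Number × Number child actor components, spaced in X and Y by Offset, which also sets each cube's XY scale.
; Each cube receives a random Z scale plus shared Z-offset bounds, back-position flag and color option through Initialization, then is stored in TempBlock.
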(fn ConstructionScript
  (Utilities|Array|Clear (Variables|Default|GetTempBlock))
  (for _index (range 0 (- (Variables|SettingsSpawn|GetNumber) 1))
    (for _index_2 (range 0 (- (Variables|SettingsSpawn|GetNumber) 1))
      (bind _returnvalue (AddComponent|AddChildActorComponent false (Math|Transform|MakeTransform (Math|Vector|MakeVector (* (Variables|SettingsSpawn|GetOffset) (Math|Conversions|ToFloat(Integer) (* _index 105))) (* (Variables|SettingsSpawn|GetOffset) (Math|Conversions|ToFloat(Integer) (* _index_2 105))) 0.0) "0, 0, 0" "1.000000,1.000000,1.000000")))
      (ChildActorComponent|SetChildActorClass _returnvalue "/Game/DynamicLevelScene/Blueprints/BP_Cube.BP_Cube_C")
      (bind _asbp_cube (Utilities|Casting|CastToBP_Cube (Variables|/Script/Engine.ChildActorComponent|GetChildActor _returnvalue)))
      (Default|Initialization _asbp_cube (Variables|SettingsSpawn|GetOffset_Z_Min) (Variables|SettingsSpawn|GetOffset_Z_Max) (Variables|SettingsSpawn|GetOffset) (Math|Random|RandomFloatinRange (Variables|SettingsCube|GetScaleMin) (Variables|SettingsCube|GetScaleMax)) (Variables|SettingsCube|GetIs%20Back%20Position) (Variables|SettingsCube|GetColor%20Option))
      (Utilities|Array|AddUnique (Variables|Default|GetTempBlock) _asbp_cube))))