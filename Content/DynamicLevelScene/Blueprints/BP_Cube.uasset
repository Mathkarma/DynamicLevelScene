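; BP_Cube is a randomly height-offset scene cube that slides toward world Z zero as a Character approaches.
; Initialization sets offset, scale, trigger sphere radius and a random color from the chosen palette via a dynamic material.
; Sphere overlap runs a looping timer that lerps height by character distance.
; With IsBackPosition the cube follows distance both ways; otherwise it only advances, destroying the sphere once it reaches zero.
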(event OnComponentBeginOverlap(Sphere)
  (params (OverlappedComponent :type Primitive%20Component%20Object%20Reference) (OtherActor :type Actor%20Object%20Reference) (OtherComp :type Primitive%20Component%20Object%20Reference) (OtherBodyIndex :type Integer) (bFromSweep :type Boolean) (SweepResult :type Hit%20Result%20Structure%20%28by%20ref%29))
  ;[0 0 0] Overlap
  (bind _ascharacter (Utilities|Casting|CastToCharacter OtherActor))
  (CallFunction|StartMove _ascharacter))

(event OnComponentEndOverlap(Sphere)
  (params (OverlappedComponent :type Primitive%20Component%20Object%20Reference) (OtherActor :type Actor%20Object%20Reference) (OtherComp :type Primitive%20Component%20Object%20Reference) (OtherBodyIndex :type Integer))
  ;[0 0 0] Overlap
  (Utilities|Casting|CastToCharacter OtherActor)
  (CallFunction|StopMove))

(event Custom|TimerMove
  (bind _sm_merged_zero (Variables|Default|GetSM_MERGED_Zero))
  (bind _returnvalue (Transformation|GetWorldLocation _sm_merged_zero))
  ;[0 0 0] Move Cube
  (bind _pawn (Variables|Default|GetPawn)
    (:then
      (if (Variables|Default|GetbIsBackPosition)
        (bind _output_get (Variables|Default|SetLastAlpha (Math|Float|MapRangeClamped (Math|Vector|Distance(Vector) (Transformation|GetWorldLocation (Variables|/Script/Engine.Actor|GetRootComponent _pawn)) (Transformation|GetWorldLocation (Variables|Default|GetSphere))) (Variables|/Script/Engine.SphereComponent|GetSphereRadius (Variables|Default|GetSphere)) (* 1.5e+02 (Variables|Default|GetScaleOffset)) 0.0 1.0) :!label _label))
        (Transformation|SetWorldLocation _sm_merged_zero (Math|Vector|MakeVector (.x _returnvalue) (.y _returnvalue) (Math|Float|Lerp (Variables|Default|GetReturn%20Value%20Z) 0.0 _output_get)) false false)
        (if (Math|Float|NearlyEqual(Float) (.z (Transformation|GetWorldLocation (Variables|Default|GetSM_MERGED_Zero))) 0.0 0.01)
          (if (not (Variables|Default|GetbIsBackPosition))
            (Utilities|Time|ClearandInvalidateTimerbyHandle (Variables|Default|GetTimer))
            (Components|DestroyComponent (Variables|Default|GetSphere))))
        (elif (> (Math|Float|MapRangeClamped (Math|Vector|Distance(Vector) (Transformation|GetWorldLocation (Variables|/Script/Engine.Actor|GetRootComponent _pawn)) (Transformation|GetWorldLocation (Variables|Default|GetSphere))) (Variables|/Script/Engine.SphereComponent|GetSphereRadius (Variables|Default|GetSphere)) (* 1.5e+02 (Variables|Default|GetScaleOffset)) 0.0 1.0) (Variables|Default|GetLastAlpha))
          (goto _label))))
    (:else)))

(event Custom|StartMove
  (params (Pawn :type Actor%20Object%20Reference))
  ;[0 0 0] Move Cube
  (Variables|Default|SetPawn Pawn)
  (bind _returnvalue (Utilities|Time|SetTimerbyEvent (delegate Custom|TimerMove) 0.012 true))
  (Variables|Default|SetTimer _returnvalue)
  (Variables|Default|SetReturn%20Value%20Z (.z (Transformation|GetWorldLocation (Variables|Default|GetSM_MERGED_Zero))))
  (Variables|Default|SetLastAlpha 0.0))

(event Custom|StopMove
  ;[0 0 0] Stop Move
  (Variables|Default|SetPawn 0)
  (Utilities|Time|ClearandInvalidateTimerbyHandle (Variables|Default|GetTimer)))

(event Custom|RandomColor
  ;[0 0 0] Random Color
  (bind _returnvalue (Rendering|Material|CreateDynamicMaterialInstance (Variables|Default|GetSM_MERGED_Zero) 0 "/Game/DynamicLevelScene/Material/CubeMaterial1.CubeMaterial1" "None" :!class /Script/Engine.PrimitiveComponent))
  (Rendering|Material|SetVectorParameterValue _returnvalue "Color" (.OutItem (Utilities|Array|Random (Utilities|Select :Index (Variables|Default|GetColorOption) :NewEnumerator0 (Utilities|Array|MakeArray "(R=1.000000,G=1.000000,B=1.000000,A=1.000000)" "(R=1.000000,G=1.000000,B=1.000000,A=1.000000)" "(R=1.000000,G=1.000000,B=1.000000,A=1.000000)" "(R=1.000000,G=1.000000,B=1.000000,A=1.000000)" "(R=1.000000,G=1.000000,B=1.000000,A=1.000000)") :NewEnumerator1 (Utilities|Array|MakeArray "(R=1.000000,G=1.000000,B=1.000000,A=1.000000)" "(R=1.000000,G=1.000000,B=1.000000,A=1.000000)" "(R=0.327778,G=1.000000,B=0.000000,A=1.000000)" "(R=1.000000,G=1.000000,B=1.000000,A=1.000000)" "(R=0.327778,G=1.000000,B=0.000000,A=1.000000)" "(R=0.327778,G=1.000000,B=0.000000,A=1.000000)" "(R=0.000000,G=0.000000,B=0.000000,A=1.000000)")))) :!class /Script/Engine.MaterialInstanceDynamic))

(fn ConstructionScript)

(fn Initialization
  (params (OffsetMin :type Float%20%28double-precision%29) (OffsetMax :type Float%20%28double-precision%29) (ScaleXY :type Float%20%28double-precision%29) (ScaleZ :type Float%20%28double-precision%29) (bIsBackPosition :type Boolean) (ColorOption :type E_ColorOption%20Enum :default "NewEnumerator0"))
  (bind _sm_merged_zero (Variables|Default|GetSM_MERGED_Zero))
  (Transformation|AddLocalOffset _sm_merged_zero (Math|Vector|MakeVector 0.0 0.0 (Math|Random|RandomFloatinRange OffsetMin OffsetMax)) false false)
  (Transformation|SetRelativeScale3D _sm_merged_zero (Math|Vector|MakeVector ScaleXY ScaleXY ScaleZ))
  (Variables|Default|SetbIsBackPosition bIsBackPosition)
  (Variables|Default|SetColorOption ColorOption)
  (CallFunction|RandomColor)
  (Variables|Default|SetScaleOffset ScaleXY)
  (Components|Sphere|SetSphereRadius (Variables|Default|GetSphere) (* 4e+02 ScaleXY) true))